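; BP_LevelHillFlappyRunner is a Flappy Runner hill piece that adds randomised background props for visual variety.
; Its construction script loops over six scene components as spawn points and randomly decides whether each gets an instance with random yaw.
; Each placement randomly sets the mesh to post or tree on one shared InstancedStaticMesh, so the last pick applies to all instances.
; The event graph holds only disabled default events.
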(fn `UserConstructionScript`
  (locals (CurrentSpawnPoint :type "SceneComponent Object Reference"))
  (`parent.UserConstructionScript`)
  (set `self.SpawnPoints` (`|MakeArray` (`self.Scene1`) (`self.Scene2`) (`self.Scene3`) (`self.Scene4`) (`self.Scene5`) (`self.Scene6`)))
  (for _array_element (`self.SpawnPoints`)
    (set `local.CurrentSpawnPoint` _array_element)
    (if (`KismetMathLibrary.RandomBool`)
      ;[0 0 0] All Completely Optional but added to randomise the background detail a little.
      ;;[1 1 1] To further randomise, select between different props
      (`StaticMeshComponent.SetStaticMesh` (`self.InstancedStaticMesh`) (select `bool` (`KismetMathLibrary.RandomBool`) :`false` "/Game/CartoonRacingPack/Models/Terrain/SM_Tree.SM_Tree" :`true` "/Game/EndlessRunnerCreator/CommonAssets/Meshes/SM_Post.SM_Post" :!type "StaticMesh Object Reference"))
      ;;[1 1 1] Props like the post look better with some random rotation to make it look less repetitive.
      (`InstancedStaticMeshComponent.AddInstance` (`self.InstancedStaticMesh`) (`KismetMathLibrary.MakeTransform` (`SceneComponent.RelativeLocation` (`local.CurrentSpawnPoint`)) (`KismetMathLibrary.MakeRotator` 0.0 0.0 (`KismetMathLibrary.RandomFloatInRange` 0.0 360.0)))))))