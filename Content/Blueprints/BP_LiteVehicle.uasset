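; BP_LiteVehicle is a drivable vehicle Blueprint that passes player input to its VehicleMovement component.
; The MoveRight and MoveForward axes set steering and throttle, and the Handbrake action sets handbrake input to true on both press and release, so nothing here clears it.
; An unconnected debug print reads slip on the first wheel through GetWheelSlip, while BeginPlay and the construction script are empty.
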(event `self.ReceiveBeginPlay`)

(event `InputAxis|MoveRight` :overrideparent false
  (params (AxisValue :type "Float (single-precision)"))
  (`MyWheeledVehicleMovementComponent.SetSteeringInput` (`self.VehicleMovement`) AxisValue))

(event `InputAxis|MoveForward`
  (params (AxisValue :type "Float (single-precision)"))
  (`MyWheeledVehicleMovementComponent.SetThrottleInput` (`self.VehicleMovement`) AxisValue))

(event `InputAction|Handbrake`
  (params (Key :type "Key Structure"))
  (bind _vehiclemovement (`self.VehicleMovement`))
  (:`Pressed`
    (`MyWheeledVehicleMovementComponent.SetHandbrakeInput` _vehiclemovement true))
  (:`Released`
    (`MyWheeledVehicleMovementComponent.SetHandbrakeInput` _vehiclemovement true)))

(fn `UserConstructionScript`)