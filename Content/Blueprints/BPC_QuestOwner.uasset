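; Quest owner component that tracks its owner's experience, gold and level, and provides interaction and mouse input helpers.
; Added experience is cumulative, raising the level and multiplying the threshold by 1.5 whenever it is reached.
; Interact sphere-traces forward from the owner and sends OnInteractMessage to the hit actor.
; Events also trigger quest saving, restore level, gold and experience (not the threshold), and toggle cursor and input mode.
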(event `self.ReceiveBeginPlay`)

(event `/Game/EasyQuests/Blueprints/BPI/BPI_Quests.ToggleMouseInput`
  (`self.Mouse Input`))

(event `AddGold`
  (params (Amount :type Integer))
  (set `self.Gold` (+ (`self.Gold`) Amount)))

(event `/Game/EasyQuests/Blueprints/BPI/BPI_Quests.ModifyGold`
  (params (Amount :type Integer))
  (`self.AddGold` Amount))

(event `/Game/EasyQuests/Blueprints/BPI/BPI_Quests.ModifyExperience`
  (params (Amount :type "Float (single-precision)"))
  (`self.AddExperience` Amount))

(event `SaveEXPGold`
  (`self.SaveQuests`))

(event `/Game/EasyQuests/Blueprints/BPI/BPI_Quests.LoadExpGoldInfo`
  (params (Level :type Integer) (Gold :type Integer) (Experience :type "Float (single-precision)") (NeededExperience :type "Float (single-precision)"))
  (set `self.Level` Level)
  (set `self.Gold` Gold)
  (set `self.Experience` Experience))

(event `AddExperience`
  (params (Amount :type "Float (double-precision)"))
  (bind _output_get (set `self.Experience` (+ (`self.Experience`) Amount)))
  (while (>= _output_get (`self.NeededExperience`))
    (`/Engine/EditorBlueprintResources/StandardMacros.IncrementInt` (`self.Level`)
      (:`  `
        (set `self.NeededExperience` (* (`self.NeededExperience`) 1.5))))))

(fn `GetExperience`
  (returns (Experience :type "Float (double-precision)"))
  (return (`self.Experience`)))

(fn `GetGold`
  (returns (TotalGold :type Integer))
  (return (`self.Gold`)))

(fn `GetLevel`
  (returns (Level :type Integer))
  (return (`self.Level`)))

(fn `GetNeededExperience`
  (returns (NeededExperience :type "Float (double-precision)"))
  (return (`self.NeededExperience`)))

(fn `Interact`
  (bind _returnvalue (`self.GetOwner`))
  (bind _returnvalue_2 (`Actor.K2_GetActorLocation` _returnvalue))
  ;[0 0 0] Handle Interaction
  (bind (_outhit _returnvalue_3) (`KismetSystemLibrary.SphereTraceSingleForObjects` _returnvalue_2 (+ _returnvalue_2 (* (`SceneComponent.GetForwardVector` (`Actor.RootComponent` _returnvalue)) (`self.InteractionRange`))) 50.0 (`|MakeArray` "ObjectTypeQuery2" "ObjectTypeQuery3" :!type "EObjectTypeQuery Enum") false (`|MakeArray` null :!type "Actor Object Reference")))
  (if _returnvalue_3
    (message `/Game/EasyQuests/Blueprints/BPI/BPI_QuestsInteraction.OnInteract` (`.HitActor` (`GameplayStatics.BreakHitResult` _outhit)) (`self.GetOwner`))))

(fn `Mouse Input`
  (bind _returnvalue (`GameplayStatics.GetPlayerController` 0))
  (if (`self.MouseVisibility`)
    (set `PlayerController.bShowMouseCursor` false _returnvalue)
    (`WidgetBlueprintLibrary.SetInputMode_GameOnly` _returnvalue)
    (set `self.MouseVisibility` false)
    (else
      (set `PlayerController.bShowMouseCursor` true _returnvalue)
      (`WidgetBlueprintLibrary.SetInputMode_GameAndUIEx` _returnvalue null)
      (set `self.MouseVisibility` true))))